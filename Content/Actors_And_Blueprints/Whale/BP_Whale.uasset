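; BP_Whale is the player-possessed whale hub, with an orbit and zoom camera that drives radial blur and room-distance material parameters.
; On first possession it creates the home menu and spawns unlocked rooms below, moving each interaction mesh to a random one of three anchors.
; Room update events trigger a HUD fade that swaps menu page and view target at full fade.
; The construction script attaches track meshes to CrawlerBed's "Track" sockets.
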(event Custom|Room%20State%20Was%20Changed
  (params (Ref%20To%20Room :type BP%20Room%20Template%20Object%20Reference))
  (bind _output_get (Variables|Default|SetNew%20Focused%20Room Ref%20To%20Room))
  (bind _assol_hud_core (Utilities|Casting|CastToSOL_HUD_Core (HUD|GetHUD (Game|GetPlayerController 0))))
  (bind _fade_widget_ref__bind_to_finished_ (Default|PlayFadeOutWidget _assol_hud_core 2.0 "PingPong"))
  (EventDispatchers|BindEventtoSwitcharoo/FULLFADE _fade_widget_ref__bind_to_finished_ (delegate Custom|Swap%20Room)))

(event Custom|Transfer)

(event Custom|Swap%20Room
  (Default|SetActiveWidgetbyRoomSelected (Variables|Default|GetWHALE%20Main%20Menu) (Variables|Default|GetNew%20Focused%20Room))
  (Game|Player|SetViewTargetwithBlend (Game|GetPlayerController 0) (select (== (stale Custom|Room%20State%20Was%20Changed _output_get) 0) self (stale Custom|Room%20State%20Was%20Changed _output_get)) 0.0 "VTBlend_Linear" 0.0 false))

(event Input|EnhancedActionEvents|EnhancedInputActionTab2
  (params (ActionValue :type Boolean) (ElapsedSeconds :type Float%20%28double-precision%29) (TriggeredSeconds :type Float%20%28double-precision%29) (InputAction :type Input%20Action%20Object%20Reference :default "/Game/Actors_And_Blueprints/PLAYER/Input/Actions/Tab2.Tab2"))
  (bind _new_focused_room (Variables|Default|GetNew%20Focused%20Room))
  (:Started
    (if (!= _new_focused_room 0)
      (Default|CallRoomUpdated _new_focused_room))))

(event Input|EnhancedActionEvents|EnhancedInputActionMouse_Click-Right
  (params (ActionValue :type Boolean) (ElapsedSeconds :type Float%20%28double-precision%29) (TriggeredSeconds :type Float%20%28double-precision%29) (InputAction :type Input%20Action%20Object%20Reference :default "/Game/Actors_And_Blueprints/PLAYER/Input/Actions/Weapons/Mouse_Click-Right.Mouse_Click-Right"))
  (:Started
    (Variables|Default|SetLeftClickHeld ActionValue :!label _label))
  (:Canceled
    (goto _label))
  (:Completed
    (goto _label)))

(event Input|EnhancedActionEvents|EnhancedInputActionMouse_Scroll
  (params (ActionValue :type Float%20%28double-precision%29) (ElapsedSeconds :type Float%20%28double-precision%29) (TriggeredSeconds :type Float%20%28double-precision%29) (InputAction :type Input%20Action%20Object%20Reference :default "/Game/Actors_And_Blueprints/PLAYER/Input/Actions/Mouse_Scroll.Mouse_Scroll"))
  (:Triggered
    (Variables|Default|SetMouseScroll ActionValue))
  (:Completed
    (Variables|Default|SetMouseScroll 0.0)))

(event Input|EnhancedActionEvents|EnhancedInputActionBackOut
  (params (ActionValue :type Boolean) (ElapsedSeconds :type Float%20%28double-precision%29) (TriggeredSeconds :type Float%20%28double-precision%29) (InputAction :type Input%20Action%20Object%20Reference :default "/Game/Actors_And_Blueprints/PLAYER/Input/Actions/Whale/BackOut.BackOut"))
  (bind _selectedroom (Variables|Default|GetSelectedRoom))
  (:Started
    (if (and ActionValue (Utilities|IsValid _selectedroom))
      (Default|CallEngaged _selectedroom false)
      (bind _returnvalue (UserInterface|CreateWidget "/Game/UI/FadeWidget.FadeWidget_C"))
      (UserInterface|Viewport|AddtoViewport _returnvalue 0)
      (Class|UserWidget|BindtoAnimationFinished _returnvalue (Variables|/Game/UI/FadeWidget.FadeWidget_C|GetFadeAnim _returnvalue) (delegate Custom|Transfer)))))

(event Collision|EventActorBeginOverlap
  (params (OtherActor :type Actor%20Object%20Reference)))

(event EventPossessed
  (params (NewController :type Controller%20Object%20Reference))
  (bind _returnvalue (Game|GetPlayerController 0))
  (bind _returnvalue_2 (Game|GetPlayerController 0))
  (Utilities|DoOnce false
    (:Completed
      (Game|Player|SetViewTargetwithBlend _returnvalue self 0.1 "VTBlend_Linear" 0.0 false)
      (Variables|/Script/Engine.PlayerController|SetbShowMouseCursor _returnvalue true)
      (Components|Activation|Activate (Variables|Default|GetStorm) false)
      (Input|AddMappingContext (PlayerController|LocalPlayerSubsystems|GetEnhancedInputLocalPlayerSubsystem (Game|GetPlayerController 0)) "/Game/Actors_And_Blueprints/PLAYER/Input/Actions/Whale/IMC_Whale.IMC_Whale" 0 "(bIgnoreAllPressedKeysUntilRelease=True,bForceImmediately=False,bNotifyUserSettings=False)")
      (Variables|/Script/Engine.PlayerController|SetbEnableMouseOverEvents _returnvalue_2 true)
      (Variables|/Script/Engine.PlayerController|SetbEnableClickEvents _returnvalue_2 true)
      (Input|EnableInput _returnvalue_2)
      (for _array_element (Actor|GetAllChildActors true)
        (Actor|SetOwner _array_element self))
      (bind _returnvalue_3 (UserInterface|CreateWidget "/Game/Worlds_And_Levels/Home/Home_Widget.Home_Widget_C" (Game|GetPlayerController 0)))
      (bind _output_get (Variables|Default|SetWHALE%20Main%20Menu _returnvalue_3))
      (EventDispatchers|BindEventtoRoomStatusChanged (EventDispatchers|CreateEvent _output_get :!event UpdateHomePAGES))
      (UserInterface|Viewport|AddtoViewport _output_get 0)
      (CallFunction|SpawnRoomsorUpdateRooms (delegate Custom|Room%20State%20Was%20Changed)))))

(event EventTick
  (params (DeltaSeconds :type Float%20%28single-precision%29))
  (bind _returnvalue (Game|GetPlayerController 0))
  (bind _springarm (Variables|Default|GetSpringArm))
  (bind _springarm_2 (Variables|Default|GetSpringArm))
  (bind (_deltax _deltay) (Class|PlayerController|GetInputMouseDelta _returnvalue))
  (bind _relativerotation (Variables|/Script/Engine.SceneComponent|GetRelativeRotation _springarm))
  (bind _returnvalue_2 (Math|Vector2D|MakeVector2D _deltax _deltay))
  (bind _returnvalue_3 (Math|Vector2D|MakeVector2D (.yaw _relativerotation) (.pitch _relativerotation)))
  (bind _returnvalue_4 (* _returnvalue_2 5e+01))
  (bind _returnvalue_5 (+ _returnvalue_3 _returnvalue_4))
  (bind _returnvalue_6 (Class|KismetMathLibrary|Vector2DInterpto _returnvalue_3 _returnvalue_5 DeltaSeconds 1.0))
  (bind (_x _y) (Math|Vector2D|BreakVector2D _returnvalue_6))
  (CallFunction|Darken)
  (Variables|/Script/Engine.SpringArmComponent|SetTargetArmLength _springarm_2 (Math|Interpolation|FInterpTo (Variables|/Script/Engine.SpringArmComponent|GetTargetArmLength _springarm_2) (+ (Variables|/Script/Engine.SpringArmComponent|GetTargetArmLength _springarm_2) (* (Variables|Default|GetMouseScroll) -5e+03)) DeltaSeconds 1.0))
  (if (Variables|Default|GetLeftClickHeld)
    (Transformation|SetRelativeRotation (Variables|Default|GetSpringArm) (Math|Rotator|MakeRotator 0.0 _y _x) false false)))

(fn ConstructionScript
  (for _array_element (Transformation|GetAllSocketNames (Variables|Default|GetCrawlerBed))
    (if (Utilities|String|Contains (Utilities|String|ToString(Name) _array_element) "Track")
      (bind _returnvalue (AddComponent|AddStaticMeshComponent false (Math|Transform|MakeTransform (.location (Transformation|GetSocketTransform (Variables|Default|GetCrawlerBed) _array_element "RTS_World")) (.rotation (Transformation|GetSocketTransform (Variables|Default|GetCrawlerBed) _array_element "RTS_World")) "1.000000,1.000000,1.000000")))
      (Components|StaticMesh|SetStaticMesh _returnvalue "/Game/Actors_And_Blueprints/AI/Enemies/Enemies/Crawler/Mesh/CrawlerTrack/StaticMeshes/CrawlerTrack.CrawlerTrack")
      (Transformation|AttachComponentToComponent _returnvalue (Variables|Default|GetCrawlerBed) _array_element "SnapToTarget" "SnapToTarget" "SnapToTarget" true)
      (Utilities|Array|Add (Variables|Default|GetPreConstructVisualizer) _returnvalue))))

(fn MouseTrace)

(fn Darken
  (bind _springarm (Variables|Default|GetSpringArm))
  (bind _targetarmlength (Variables|/Script/Engine.SpringArmComponent|GetTargetArmLength _springarm))
  (Rendering|Material|SetScalarParameterValue "/Game/Actors_And_Blueprints/Whale/MPC_RoomData.MPC_RoomData" "Distance" (Math|Float|MapRangeClamped _targetarmlength 2e+03 3e+03 0.3 1.0) :!class /Script/Engine.KismetMaterialLibrary)
  (Rendering|Material|SetScalarParameterValue "/Game/VFX/MPC_Radial_Blur.MPC_Radial_Blur" "Value" (Math|Float|MapRangeClamped _targetarmlength 2e+03 3e+03 1.0 0.3) :!class /Script/Engine.KismetMaterialLibrary))

(fn SpawnRoomsorUpdateRooms
  (params (Room%20Updated%20Event :type Delegate%20%28by%20ref%29))
  (bind (_keypin _valuepin) (Utilities|Map|ForEachLoop(Map) (Variables|Default|GetUnlocked%20Rooms%20To%20Spawn))
    (:then
      (if _valuepin
        (bind _output_get (LocalVariables|SetLooped%20Room _keypin))
        (if (Utilities|IsValidClass (Utilities|ResolveSoftReference _output_get))
          (LocalVariables|SetFound%20Hard%20Class (Utilities|ResolveSoftReference (LocalVariables|GetLooped%20Room)))
          (else
            (bind _returnvalue (Utilities|LoadClassAssetBlocking (LocalVariables|GetLooped%20Room)))
            (LocalVariables|SetFound%20Hard%20Class (.AsBP%20Room%20Template (Utilities|Casting|CastToBP_Room_TemplateClass _returnvalue)))))
        (bind _returnvalue_2 (Game|SpawnActorfromClass (LocalVariables|GetFound%20Hard%20Class) (Math|Transform|MakeTransform "0.000000,0.000000,-5000.000000" "0, 0, 0" "1.000000,1.000000,1.000000") "Undefined" "MultiplyWithRoot" self 0))
        (bind _output_get_2 (LocalVariables|SetConstructed%20Room _returnvalue_2))
        (EventDispatchers|BindEventtoRoomUpdated _output_get_2 Room%20Updated%20Event)
        (Transformation|SetWorldTransform (Variables|/Game/Actors_And_Blueprints/Whale/Dollhouse/Rooms/BP_Room_Template.BP_Room_Template_C|GetRoom%20Interaction%20Mesh (LocalVariables|GetConstructed%20Room)) (Transformation|GetWorldTransform (Utilities|Select :Index (Math|Random|RandomIntegerinRange 0 2) :Option%200 (Variables|Default|GetRoom%20Int%20Mesh:%20Crafter) :Option%201 (Variables|Default|GetRoom%20int%20Mesh:%20Whale%20Heart) :Option%202 (Variables|Default|GetRoom%20Int%20Mesh:%20Store))) false true)
        (Default|CallRoomStatusChanged (LocalVariables|GetConstructed%20Room) true)
        (Development|PrintString (Utilities|String|ToString(Text) (Utilities|Text|FormatText "ROOM CONSTRUCTED 
{Room} 
Found? {Val}" (LocalVariables|GetConstructed%20Room))) true true "(R=1.000000,G=0.128238,B=0.863214,A=1.000000)" 1e+01)))
    (:CompletedPin
      (return))))