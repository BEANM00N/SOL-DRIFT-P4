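; Clickable room icon in the whale dollhouse that moves the player's view into its associated room.
; On BeginPlay it spawns a hidden room far below the origin and applies an X-ray overlay material that changes color on hover.
; Clicking records the room on the owning BP_Whale, stops its tick, disables mouse events and plays a fade.
; After the fade it switches view target, reveals and engages the room, and adjusts opacity and radial-blur parameter collections.
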(event OnBeginCursorOver(Mesh)
  (params (TouchedComponent :type Primitive%20Component%20Object%20Reference))
  (Rendering|Material|SetVectorParameterValue (Variables|Default|GetOverlayMaterial) "Color" "(R=0.814847,G=0.814847,B=0.814847,A=1.000000)" :!class /Script/Engine.MaterialInstanceDynamic))

(event OnEndCursorOver(Mesh)
  (params (TouchedComponent :type Primitive%20Component%20Object%20Reference))
  (Rendering|Material|SetVectorParameterValue (Variables|Default|GetOverlayMaterial) "Color" "(R=1.000000,G=0.351533,B=0.000000,A=1.000000)" :!class /Script/Engine.MaterialInstanceDynamic))

(event OnClicked(Mesh)
  (params (TouchedComponent :type Primitive%20Component%20Object%20Reference) (ButtonPressed :type Key%20Structure :default "None"))
  (bind _returnvalue (Game|GetPlayerController 0))
  (bind _asbp_whale (Utilities|Casting|CastToBP_Whale (Components|GetOwner)))
  (Variables|/Game/Actors_And_Blueprints/Whale/BP_Whale.BP_Whale_C|SetSelectedRoom _asbp_whale (Variables|Default|GetAssociatedRoom))
  (Actor|Tick|SetActorTickEnabled _asbp_whale)
  (bind _returnvalue_2 (UserInterface|CreateWidget "/Game/UI/FadeWidget.FadeWidget_C"))
  (UserInterface|Viewport|AddtoViewport _returnvalue_2 0)
  (Class|UserWidget|BindtoAnimationFinished _returnvalue_2 (Variables|/Game/UI/FadeWidget.FadeWidget_C|GetFadeAnim _returnvalue_2) (delegate Custom|Transfer))
  (Variables|/Script/Engine.PlayerController|SetbEnableClickEvents _returnvalue false)
  (Variables|/Script/Engine.PlayerController|SetbEnableMouseOverEvents _returnvalue false))

(event Custom|Transfer
  (bind _associatedroom (Variables|Default|GetAssociatedRoom))
  (Game|Player|SetViewTargetwithBlend (Game|GetPlayerController 0) (Variables|Default|GetAssociatedRoom) 0.0 "VTBlend_Linear" 0.0 false)
  (Rendering|Material|SetScalarParameterValue "/Game/Actors_And_Blueprints/Whale/MPC_RoomData.MPC_RoomData" "Opacity" 0.0 :!class /Script/Engine.KismetMaterialLibrary)
  (bind _returnvalue (UserInterface|CreateWidget "/Game/UI/FadeWidget.FadeWidget_C" 0 true))
  (UserInterface|Viewport|AddtoViewport _returnvalue 0)
  (Rendering|SetActorHiddenInGame _associatedroom false)
  (Default|CallEngaged _associatedroom true)
  (Rendering|Material|SetScalarParameterValue "/Game/VFX/MPC_Radial_Blur.MPC_Radial_Blur" "Value" 0.5 :!class /Script/Engine.KismetMaterialLibrary))

(event EventBeginPlay
  (bind _returnvalue (Rendering|Material|CreateDynamicMaterialInstance "/Game/Actors_And_Blueprints/Whale/MI_Xray.MI_Xray" "None" "None" :!class /Script/Engine.KismetMaterialLibrary))
  (Rendering|Material|SetOverlayMaterial (Variables|Default|GetMesh) _returnvalue :!class /Script/Engine.MeshComponent)
  (Variables|Default|SetOverlayMaterial _returnvalue)
  (bind _returnvalue_2 (Game|SpawnActorfromClass (Variables|Default|GetRoomClass) (Math|Transform|MakeTransform "0.000000,0.000000,-5000.000000" "0, 0, 0" "1.000000,1.000000,1.000000") "Undefined" "MultiplyWithRoot" 0 0))
  (bind _output_get (Variables|Default|SetAssociatedRoom (.AsBP%20Room%20Template (Utilities|Casting|CastToBP_Room_Template _returnvalue_2))))
  (Rendering|SetActorHiddenInGame _output_get true))

(event Collision|EventActorBeginOverlap
  (params (OtherActor :type Actor%20Object%20Reference)))

(event EventTick
  (params (DeltaSeconds :type Float%20%28single-precision%29)))

(fn ConstructionScript)