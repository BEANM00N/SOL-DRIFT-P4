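; BP_Room_Template is a dollhouse room that highlights on mouse hover and reports clicks through CallRoomUpdated.
; BeginPlay puts a dynamic MI_Xray overlay on the interaction mesh, and cursor events switch its color between orange and light gray.
; Transfer makes the room the view target and zeroes MPC_RoomData opacity, but its fade-widget binding and a room-scene visibility call sit in unconnected nodes.
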(event OnBeginCursorOver(RoomInteractionMesh)
  (params (TouchedComponent :type Primitive%20Component%20Object%20Reference))
  (Rendering|Material|SetVectorParameterValue (Variables|Default|GetOverlayMaterial) "Color" "(R=0.814847,G=0.814847,B=0.814847,A=1.000000)" :!class /Script/Engine.MaterialInstanceDynamic))

(event OnEndCursorOver(RoomInteractionMesh)
  (params (TouchedComponent :type Primitive%20Component%20Object%20Reference))
  (Rendering|Material|SetVectorParameterValue (Variables|Default|GetOverlayMaterial) "Color" "(R=1.000000,G=0.351533,B=0.000000,A=1.000000)" :!class /Script/Engine.MaterialInstanceDynamic))

(event OnClicked(RoomInteractionMesh)
  (params (TouchedComponent :type Primitive%20Component%20Object%20Reference) (ButtonPressed :type Key%20Structure :default "None"))
  (Default|CallRoomUpdated self))

(event Custom|Transfer
  (Game|Player|SetViewTargetwithBlend (Game|GetPlayerController 0) self 0.0 "VTBlend_Linear" 0.0 false)
  (Rendering|Material|SetScalarParameterValue "/Game/Actors_And_Blueprints/Whale/MPC_RoomData.MPC_RoomData" "Opacity" 0.0 :!class /Script/Engine.KismetMaterialLibrary))

(event EventBeginPlay
  (bind _returnvalue (Rendering|Material|CreateDynamicMaterialInstance "/Game/Actors_And_Blueprints/Whale/MI_Xray.MI_Xray" "None" "None" :!class /Script/Engine.KismetMaterialLibrary))
  (Rendering|Material|SetOverlayMaterial (Variables|Default|GetRoom%20Interaction%20Mesh) _returnvalue :!class /Script/Engine.MeshComponent)
  (Variables|Default|SetOverlayMaterial _returnvalue))

(fn ConstructionScript)