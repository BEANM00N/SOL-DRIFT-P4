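; BP_Eye is an eye actor for dollhouse rooms that turns to follow the player's mouse cursor.
; On BeginPlay it binds to the Engaged event of its parent BP_Room_Template, and its SetState event switches ticking on or off.
; Each Tick deprojects the cursor into world space and uses a look-at rotation to aim at a point a fixed distance along that ray.
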(event Custom|SetState
  (params (State :type Boolean))
  (Actor|Tick|SetActorTickEnabled State))

(event EventBeginPlay
  (EventDispatchers|BindEventtoEngaged (.AsBP%20Room%20Template (Utilities|Casting|CastToBP_Room_Template (Actor|GetParentActor))) (EventDispatchers|CreateEvent :!event Custom|SetState)))

(event Collision|EventActorBeginOverlap
  (params (OtherActor :type Actor%20Object%20Reference)))

(event EventTick
  (params (DeltaSeconds :type Float%20%28single-precision%29))
  (bind _returnvalue (Game|GetPlayerController 0))
  (bind (_locationx _locationy) (Game|Player|GetMousePosition _returnvalue))
  (bind (_worldposition _worlddirection) (Class|GameplayStatics|DeprojectScreentoWorld _returnvalue (Math|Vector2D|MakeVector2D _locationx _locationy)))
  (Transformation|SetActorRotation (Math|Rotator|FindLookatRotation (Transformation|GetActorLocation) (+ _worldposition (* _worlddirection 2e+02)))))

(fn ConstructionScript)