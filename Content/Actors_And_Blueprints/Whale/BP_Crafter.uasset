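; BP_Crafter is a clickable crafter room owned by BP_Whale that the player's view blends to when selected.
; It applies a dynamic X-ray overlay material to its mesh and changes that material's color on cursor hover.
; Clicking registers it as the whale's SelectedRoom, zeroes the Opacity parameter in MPC_RoomData, blends the view to itself and disables player click and hover events.
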(event OnBeginCursorOver(Mesh)
  (params (TouchedComponent :type Primitive%20Component%20Object%20Reference))
  (Rendering|Material|SetVectorParameterValue (Variables|Default|GetOverlayMaterial) "Color" "(R=0.814847,G=0.814847,B=0.814847,A=1.000000)" :!class /Script/Engine.MaterialInstanceDynamic))

(event OnEndCursorOver(Mesh)
  (params (TouchedComponent :type Primitive%20Component%20Object%20Reference))
  (Rendering|Material|SetVectorParameterValue (Variables|Default|GetOverlayMaterial) "Color" "(R=1.000000,G=0.254918,B=0.000000,A=1.000000)" :!class /Script/Engine.MaterialInstanceDynamic))

(event OnClicked(Mesh)
  (params (TouchedComponent :type Primitive%20Component%20Object%20Reference) (ButtonPressed :type Key%20Structure :default "None"))
  (bind _returnvalue (Game|GetPlayerController 0))
  (bind _self self)
  (bind _asbp_whale (Utilities|Casting|CastToBP_Whale (Components|GetOwner)))
  (Variables|/Game/Actors_And_Blueprints/Whale/BP_Whale.BP_Whale_C|SetSelectedRoom _asbp_whale _self)
  (Rendering|Material|SetScalarParameterValue "/Game/Actors_And_Blueprints/Whale/MPC_RoomData.MPC_RoomData" "Opacity" 0.0 :!class /Script/Engine.KismetMaterialLibrary)
  (Game|Player|SetViewTargetwithBlend (Game|GetPlayerController 0) _self 0.5 "VTBlend_Linear" 0.0 false)
  (Variables|/Script/Engine.PlayerController|SetbEnableClickEvents _returnvalue false)
  (Variables|/Script/Engine.PlayerController|SetbEnableMouseOverEvents _returnvalue false))

(event EventBeginPlay
  (bind _returnvalue (Rendering|Material|CreateDynamicMaterialInstance "/Game/Actors_And_Blueprints/Whale/MI_Xray.MI_Xray" "None" "None" :!class /Script/Engine.KismetMaterialLibrary))
  (Rendering|Material|SetOverlayMaterial (Variables|Default|GetMesh) _returnvalue :!class /Script/Engine.MeshComponent)
  (Variables|Default|SetOverlayMaterial _returnvalue))

(event Collision|EventActorBeginOverlap
  (params (OtherActor :type Actor%20Object%20Reference)))

(event EventTick
  (params (DeltaSeconds :type Float%20%28single-precision%29)))

(fn ConstructionScript)