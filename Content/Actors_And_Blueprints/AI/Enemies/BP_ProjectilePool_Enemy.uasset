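; BP_ProjectilePool_Enemy is an object pool that supplies reusable projectiles for enemies.
; On BeginPlay it pre-spawns PoolSize actors of PooledProjectileClass and marks each as not in use.
; SpawnFromPool linearly searches for the first free projectile, moves it to the requested transform, activates it with an owner and returns it.
; The pool never grows, so no projectile is activated when all are busy.
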(event Custom|Initialize%20Pool
  (params (Owner :type Actor%20Object%20Reference))
  (for _index (range 1 (Variables|Default|GetPoolSize))
    (bind _returnvalue (Game|SpawnActorfromClass (Variables|Default|GetPooledProjectileClass) (Math|Transform|MakeTransform "0, 0, 0" "0, 0, 0" "1.000000,1.000000,1.000000") "Undefined" "MultiplyWithRoot" Owner 2.0 0))
    (Utilities|Array|AddUnique (Variables|Default|GetPooledProjectiles) _returnvalue)
    (CallFunction|SetinUse _returnvalue false)))

(event EventBeginPlay
  (CallFunction|InitializePool))

(event EventTick
  (params (DeltaSeconds :type Float%20%28single-precision%29)))

(fn FindFirstAvailableProjectile
  (for _array_element (Variables|Default|GetPooledProjectiles)
    (if (not (Variables|Default|GetInUse _array_element))
      (return _array_element))))

(fn SpawnfromPool
  (params (Transform :type Transform) (Owner :type Actor%20Object%20Reference))
  (bind _pooledprojectile (CallFunction|FindFirstAvailableProjectile))
  (Utilities|IsValid _pooledprojectile
    (:Is%20Valid
      (Transformation|SetActorTransform _pooledprojectile Transform)
      (CallFunction|SetinUse _pooledprojectile true Owner)
      (return _pooledprojectile))))