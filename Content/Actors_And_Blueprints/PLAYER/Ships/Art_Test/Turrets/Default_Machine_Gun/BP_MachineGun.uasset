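; Player ship machine gun turret, a child weapon Blueprint that handles automatic fire, barrel spool, heat and reloading.
; Trigger input starts looping spool and self-rearming fire timers; the fire interval lerps on spool but both endpoints match.
; Releasing the trigger or reloading drains heat on a timer, and empty ammo triggers a timed reload that resumes firing if input is held.
; Helper functions spawn the socketed skeletal mesh with twin Niagara muzzle flashes and accumulate heat.
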(event Custom|Begin%20Firing
  (if (Math|Boolean|ANDBoolean (Variables|Default|GetPlayer%20Input%20State) (Variables|Default|GetCan%20Fire?) (not (Variables|Default|GetWeapon%20Out%20Of%20Ammo)))
    (Default|CallWeaponWasFired)
    (bind _returnvalue (Utilities|Time|SetTimerbyEvent (delegate Custom|Begin%20Firing) (Math|Float|Lerp 0.15 0.15 (Variables|Default|GetWhirr%20Current))))
    (Variables|Default|SetWeapon%20Firing%20Timer _returnvalue)
    (else
      (Utilities|Time|ClearandInvalidateTimerbyHandle (Variables|Default|GetWeapon%20Firing%20Timer))
      (Development|PrintString "CANCEL"))))

(event Custom|Reduce%20Ammo
  (bind _weapon_out_of_ammo (Variables|Default|GetWeapon%20Out%20Of%20Ammo))
  ;[0 0 0 0.5] Reduce Weapon Ammo
  (|CallParentFunction)
  (if _weapon_out_of_ammo
    (Default|CallWeaponReload _weapon_out_of_ammo)))

(event Custom|Weapon%20Reloaded
  ;[0 0 0 0.5] Reload Weapon
  (|CallParentFunction)
  (if (Variables|Default|GetPlayer%20Input%20State)
    (CallFunction|FireOverRide)))

(event Custom|Drain%20HEAT
  ;[0.15 0.15 0.15 0.5] Drain HEAT
  (bind _output_get (Variables|Default|SetCurrent%20HEAT (Math|Interpolation|FInterptoConstant (Variables|Default|GetCurrent%20HEAT) 0.0 (Utilities|Time|GetWorldDeltaSeconds) (Math|Float|SelectFloat 0.1 (Variables|Default|GetCooling%20Rate%20%28Spooled%29) (and (Variables|Default|GetReloading%20State) (not (Variables|Default|GetPlayer%20Input%20State)))))))
  (Default|CallHeatStateChange _output_get)
  (if (== _output_get 0.0)
    (Utilities|Time|ClearandInvalidateTimerbyHandle (Variables|Default|GetHEAT%20Drain%20Timer))))

(event Custom|Update%20Spooling
  (bind _player_input_state (Variables|Default|GetPlayer%20Input%20State))
  (bind _output_get (Variables|Default|SetWhirr%20Current (Math|Interpolation|FInterptoConstant (Variables|Default|GetWhirr%20Current) (Math|Float|SelectFloat 1.0 0.0 _player_input_state) 0.1 (Math|Float|SelectFloat (Variables|Default|GetCooling%20Rate%20%28Spooled%29) (Variables|Default|GetCooling%20Rate) _player_input_state))))
  (if (or (== _output_get 0.0) (== _output_get 1.0))
    (Utilities|Time|ClearandInvalidateTimerbyHandle (Variables|Default|GetSpool%20Timer))))

(event Custom|Begin%20Draining%20Heat
  ;[0.15 0.15 0.15 0.5] Drain HEAT
  (Development|PrintString "DRAIN")
  (bind _returnvalue (Utilities|Time|SetTimerbyEvent (delegate Custom|Drain%20HEAT) 0.01 true false (Math|Float|SelectFloat 0.0 0.5 (Utilities|Time|IsValidTimerHandle (Variables|Default|GetHEAT%20Drain%20Timer)))))
  (Variables|Default|SetHEAT%20Drain%20Timer _returnvalue))

(event Custom|TempCameraShake
  (Camera|PlayWorldCameraShake "/Game/VFX/Camera_Shakes/ChainRaptorTemp.ChainRaptorTemp_C" "0, 0, 0" 1e+04 5e+04))

(event EventBeginPlay
  (|CallParentFunction)
  (Variables|Default|SetCan%20Fire? true))

(event EventFireOverRide
  (if (Variables|Default|GetPlayer%20Input%20State)
    _
    (else
      (CallFunction|BeginDrainingHeat)))
  (bind _returnvalue (Utilities|Time|SetTimerbyEvent (delegate Custom|Update%20Spooling) 0.01 true))
  (Variables|Default|SetSpool%20Timer _returnvalue)
  (bind _returnvalue_2 (Utilities|Time|SetTimerbyEvent (delegate Custom|Begin%20Firing) (Math|Float|Lerp 0.15 0.15 (Variables|Default|GetWhirr%20Current))))
  (Variables|Default|SetWeapon%20Firing%20Timer _returnvalue_2))

(event EventPlayerAttemptingWeaponTrigger
  (params (Input%20Status%20From%20Controller :type Boolean))
  (|CallParentFunction Input%20Status%20From%20Controller)
  (if (Variables|Default|GetPlayer%20Input%20State)
    _
    (else
      (CallFunction|BeginDrainingHeat)))
  (bind _returnvalue (Utilities|Time|SetTimerbyEvent (delegate Custom|Update%20Spooling) 0.01 true))
  (Variables|Default|SetSpool%20Timer _returnvalue)
  (bind _returnvalue_2 (Utilities|Time|SetTimerbyEvent (delegate Custom|Begin%20Firing) (Math|Float|Lerp 0.15 0.15 (Variables|Default|GetWhirr%20Current))))
  (Variables|Default|SetWeapon%20Firing%20Timer _returnvalue_2))

(event EventWeaponReloadStateEvent
  (params (Reload%20Event :type Boolean))
  ;[0 0 0 0.5] Reload Weapon
  (if (!= (Variables|Default|GetAmmo%20Reserves%20%28Current%29) 0)
    (|CallParentFunction Reload%20Event)
    (if Reload%20Event
      (bind _returnvalue (Utilities|Time|SetTimerbyEvent (delegate Custom|Weapon%20Reloaded) (Variables|Default|GetReload%20Time)))
      (Variables|Default|SetReload%20Timer%20Handle _returnvalue)
      (CallFunction|BeginDrainingHeat))))

(event EventSetWeaponEquipState
  (params (Equip%20State%20To%20Set :type Boolean))
  (|CallParentFunction Equip%20State%20To%20Set)
  (if (== (Variables|Default|GetWhirr%20Current) 1.0)
    (bind _returnvalue (Utilities|Time|SetTimerbyEvent (delegate Custom|Update%20Spooling) 0.01 true))
    (Variables|Default|SetSpool%20Timer _returnvalue)
    (bind _returnvalue_2 (Utilities|Time|SetTimerbyEvent (delegate Custom|Begin%20Firing) (Math|Float|Lerp 0.15 0.15 (Variables|Default|GetWhirr%20Current))))
    (Variables|Default|SetWeapon%20Firing%20Timer _returnvalue_2)))

(fn ConstructionScript
  (|CallParentFunction)
  (EventDispatchers|BindEventtoWeaponWasFired (EventDispatchers|CreateEvent :!event Custom|TempCameraShake)))

(fn AddNiagraVFXtoWeaponMesh
  (params (WeaponMesh :type Skeletal%20Mesh%20Component%20Object%20Reference))
  (bind _returnvalue (AddComponent|AddNiagaraComponent (Components|GetOwner WeaponMesh) false (Math|Transform|MakeTransform "0, 0, 0" "0, 0, 0" (Math|Conversions|ToVector(Float) 0.0035))))
  (Class|NiagaraComponent|SetAsset _returnvalue "/Game/Actors_And_Blueprints/PLAYER/Equipment_Modules/Weapons/Chain_Raptor/MuzzleFlashes/Muzzle_Flash.Muzzle_Flash" true)
  (Transformation|AttachComponentToComponent _returnvalue WeaponMesh "MuzzleSocket" "SnapToTarget" "SnapToTarget" "KeepRelative" true)
  (Utilities|Array|Add (Variables|Default|GetMuzzleFlashArray) _returnvalue)
  (bind _returnvalue_2 (AddComponent|AddNiagaraComponent false))
  (Transformation|AttachComponentToComponent _returnvalue_2 WeaponMesh "Laser" "SnapToTarget" "SnapToTarget" "KeepRelative" true)
  (bind _returnvalue_3 (AddComponent|AddNiagaraComponent (Components|GetOwner WeaponMesh) false (Math|Transform|MakeTransform "0, 0, 0" "0, 0, 0" (Math|Conversions|ToVector(Float) 0.0035))))
  (Class|NiagaraComponent|SetAsset _returnvalue_3 "/Game/Actors_And_Blueprints/PLAYER/Equipment_Modules/Weapons/Chain_Raptor/MuzzleFlashes/Muzzle_Flash.Muzzle_Flash" true)
  (Transformation|AttachComponentToComponent _returnvalue_3 WeaponMesh "MuzzleSocket1" "SnapToTarget" "SnapToTarget" "KeepRelative" true)
  (Utilities|Array|Add (Variables|Default|GetMuzzleFlashArray) _returnvalue_3)
  (bind _returnvalue_4 (AddComponent|AddNiagaraComponent false))
  (Transformation|AttachComponentToComponent _returnvalue_4 WeaponMesh "Laser1" "SnapToTarget" "SnapToTarget" "KeepRelative" true)
  (return))

(fn GenerateHEAT
  (bind _heat_drain_timer (Variables|Default|GetHEAT%20Drain%20Timer))
  (if (Utilities|Time|IsValidTimerHandle _heat_drain_timer)
    (Utilities|Time|ClearandInvalidateTimerbyHandle _heat_drain_timer))
  (bind _output_get (Variables|Default|SetCurrent%20HEAT (Math|Float|Clamp(Float) (+ (Variables|Default|GetHeat%20gen) (Variables|Default|GetCurrent%20HEAT)))))
  (Default|CallHeatStateChange _output_get)
  (if (== _output_get 1.0)
    _))

(fn SpawnWeaponMesh
  (params (Socket%20To%20Attach%20To :type Name :default "None"))
  (bind _returnvalue (Utilities|Name|MakeLiteralName "TurretSocket"))
  (bind _weapon_meshes_reference (Variables|Default|GetWeapon%20Meshes%20Reference))
  (bind _returnvalue_2 (AddComponent|AddSkeletalMeshComponent false (Math|Transform|MakeTransform (Transformation|GetWorldLocation (Variables|Default|GetDefaultSceneRoot)) "0.000000,0.000000,-90.000000" (Math|Conversions|ToVector(Float) 0.012))))
  (Variables|Default|SetWeaponMeshComp _returnvalue_2)
  (Components|SkeletalMesh|SetAnimInstanceClass _returnvalue_2 (Variables|Default|GetAnimation%20Class))
  (bind _avalaible_mesh_to_attach_to (Class|SOLWeaponsInterface|ReturnSceneComponenttoAttachto(Message) (Components|GetOwner)))
  (bind _returnvalue_3 (Utilities|Array|Add _weapon_meshes_reference _returnvalue_2))
  (Components|SkeletalMesh|SetSkeletalMeshAsset (Utilities|Array|Get(acopy) _weapon_meshes_reference _returnvalue_3) (Utilities|Struct|BreakWeaponData (Variables|Default|GetWeapon%20Data)))
  (Utilities|Map|Add (Variables|Default|GetCreated%20Weapons%20Array%20With%20Sockets) _returnvalue (Utilities|Array|Get(acopy) _weapon_meshes_reference _returnvalue_3))
  (Transformation|AttachComponentToComponent (Utilities|Array|Get(acopy) _weapon_meshes_reference _returnvalue_3) _avalaible_mesh_to_attach_to _returnvalue "SnapToTarget" "KeepRelative" "KeepRelative" true)
  (CallFunction|AddNiagraVFXtoWeaponMesh (Utilities|Array|Get(acopy) _weapon_meshes_reference _returnvalue_3))
  (Rendering|Components|SetLightingChannels (Variables|Default|GetWeaponMeshComp) false true false))