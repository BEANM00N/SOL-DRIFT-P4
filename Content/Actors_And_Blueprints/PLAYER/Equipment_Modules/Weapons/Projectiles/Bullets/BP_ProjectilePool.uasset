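; Projectile pool for a weapon, which pre-spawns bullet actors when owned by a WeaponSystemBASE.
; Shortly after BeginPlay it binds to the owning weapon's fired event and fills an array with 30 instances of the pooled projectile class.
; FindNextProjectile selects an entry by the current magazine index, which nothing here updates.
; SpawnFromPool is empty and GetSightCone returns a zero vector, so firing from the pool is unfinished.
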(event EventBeginPlay
  (Utilities|FlowControl|Delay 0.2)
  (bind _asweapon_system_base (Utilities|Casting|CastToWeaponSystemBASE (Components|GetOwner)))
  (bind _output_get (Variables|Default|SetOwning%20Weapon _asweapon_system_base))
  (EventDispatchers|BindEventtoWeaponWasFired _output_get (EventDispatchers|CreateEvent :!event SpawnfromPool))
  (bind _output_get_2 (Variables|Default|SetPoolSize 30))
  (for _index (range 1 _output_get_2)
    (bind _returnvalue (Game|SpawnActorfromClass (Variables|Default|GetPooledProjectileClass) (Math|Transform|MakeTransform "0, 0, 0" "0, 0, 0" "1.000000,1.000000,1.000000") "Undefined" "MultiplyWithRoot" 0 0 0))
    (Utilities|Array|Add (Variables|Default|GetPooledProjectiles) _returnvalue)))

(fn FindNextProjectile
  (bind _current_projectile_in_mag (Variables|Default|GetCurrent%20Projectile%20In%20Mag))
  (Variables|Default|SetProjectile%20To%20Fire (Utilities|Array|Get(acopy) (Variables|Default|GetPooledProjectiles) _current_projectile_in_mag))
  (return (< _current_projectile_in_mag 0)))

(fn SpawnfromPool)

(fn GetSightCone
  (return "0, 0, 0"))