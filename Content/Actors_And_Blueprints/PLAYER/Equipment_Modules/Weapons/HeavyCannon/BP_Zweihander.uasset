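; BP_Zweihander is a player heavy cannon weapon module, built on a parent weapon class that handles trigger input and animation setup.
; Its VFX setup scans mesh socket names, attaching stored muzzle flash Niagara components to "Muzzle" sockets and Niagara components, spotlight and decal to "Laser" sockets.
; Its projectile override plays a camera shake and pitch-randomized sound, then spawns an Enemy-targeting CannonBullet from MuzzleSocket.
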(event EventBeginPlay
  (|CallParentFunction))

(event EventPlayerAttemptingWeaponTrigger
  (params (Input%20Status%20From%20Controller :type Boolean))
  (|CallParentFunction Input%20Status%20From%20Controller))

(fn ConstructionScript
  (|CallParentFunction))

(fn AddNiagraVFXtoWeaponMesh
  (params (WeaponMesh :type Skeletal%20Mesh%20Component%20Object%20Reference))
  ;[0.15 0.15 0.15 0.5] Add Muzzle Flash
  (for _array_element (Transformation|GetAllSocketNames (Variables|Default|GetWeapon%20SKM))
    (if (Utilities|String|Contains (Utilities|String|ToString(Name) _array_element) "Muzzle")
      (bind _returnvalue (AddComponent|AddNiagaraComponent false (Math|Transform|MakeTransform "0, 0, 0" "0, 0, 0" (Math|Conversions|ToVector(Float) 0.0105))))
      (Class|NiagaraComponent|SetAsset _returnvalue "/Game/VFX/MuzzleFlashes/Muzzle_Flash.Muzzle_Flash" true)
      (Transformation|AttachComponentToComponent _returnvalue (Variables|Default|GetWeapon%20SKM) _array_element "SnapToTarget" "SnapToTarget" "KeepRelative" true)
      (Utilities|Array|Add (Variables|Default|GetMuzzleFlashArray) _returnvalue)))
  ;[0.15 0.15 0.15 0.5] Add Lasers
  (for _array_element_2 (Transformation|GetAllSocketNames (Variables|Default|GetWeapon%20SKM))
    (if (Utilities|String|Contains (Utilities|String|ToString(Name) _array_element_2) "Laser")
      (bind _returnvalue_2 (AddComponent|AddNiagaraComponent false))
      (Transformation|AttachComponentToComponent _returnvalue_2 (Variables|Default|GetWeapon%20SKM) _array_element_2 "SnapToTarget" "SnapToTarget" "KeepRelative" true)
      (Transformation|AttachComponentToComponent (Variables|Default|GetSpotLight) (Variables|Default|GetWeapon%20SKM) _array_element_2 "SnapToTarget" "SnapToTarget" "KeepRelative" true)
      (Transformation|AttachComponentToComponent (Variables|Default|GetDecal) (Variables|Default|GetWeapon%20SKM) _array_element_2 "SnapToTarget" "SnapToTarget" "KeepRelative" true))))

(fn InitialiseAnimation
  (|CallParentFunction))

(fn SpawnEntityProjectile
  (params (Mesh%20Reference%20To%20Spawn%20From :type Scene%20Component%20Object%20Reference) (SocketMethodTemp :type Name :default "None"))
  (bind _weapon_skm (Variables|Default|GetWeapon%20SKM))
  (bind _returnvalue (Transformation|GetSocketTransform _weapon_skm "MuzzleSocket" "RTS_World"))
  (Camera|PlayWorldCameraShake "/Game/VFX/Camera_Shakes/GrenadeLauncher.GrenadeLauncher_C" "0, 0, 0" 1e+04 5e+04)
  (Audio|PlaySound2D "/Game/Actors_And_Blueprints/PLAYER/Equipment_Modules/Weapons/HeavyCannon/AC_SFX.AC_SFX" (Math|Random|RandomFloatinRange 0.9 1.1) (Math|Random|RandomFloatinRange 1.9 2.1) 0.0 0 0)
  (Game|SpawnActorfromClass "/Game/Actors_And_Blueprints/PLAYER/Equipment_Modules/Weapons/Projectiles/Bullets/CannonBullet.CannonBullet_C" (Math|Transform|MakeTransform (.location _returnvalue) (.rotation _returnvalue) "1.000000,1.000000,1.000000") "Undefined" "MultiplyWithRoot" 0 5.0 0 "Enemy" 1e+01 "Player" 0))