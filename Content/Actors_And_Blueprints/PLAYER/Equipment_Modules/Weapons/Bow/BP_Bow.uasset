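; Player bow weapon, derived from a parent weapon class, that is drawn while the trigger is held and fires on release.
; A timer drives DrawPower, feeding the animation instance and shrinking hip and ADS accuracy values from their saved bases.
; SpawnFLECSProjectile spawns a Bolt actor carrying DrawPower, aimed by a crosshair screen trace.
; Other overrides attach muzzle and laser effects by socket name and spawn shotgun-style twelve-projectile entity volleys.
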(event Custom|DUD)

(event EventBeginPlay
  (|CallParentFunction)
  (Variables|Default|SetRoot%20Accuracy (Variables|Default|GetStandard%20Accuracy))
  (Variables|Default|SetRoot%20ADS%20Accuracy (Variables|Default|GetADS%20Accuracy)))

(event EventWeaponFiringToggle
  (params (Toggle :type Boolean))
  (Development|PrintText (Utilities|Text|FormatText "BOOM {S}" Toggle))
  (if Toggle
    (bind _returnvalue (Utilities|Time|SetTimerbyEvent (delegate Custom|DUD) 1.5))
    (Variables|Default|SetDrawLength _returnvalue)
    (Variables|Default|SetDrawingString true)
    (else
      (Utilities|Time|ClearandInvalidateTimerbyHandle (Variables|Default|GetDrawLength))
      (Variables|Default|SetDrawingString false)
      (Default|CallWeaponWasFired))))

(event EventTick
  (params (DeltaSeconds :type Float%20%28single-precision%29))
  (bind _drawlength (Variables|Default|GetDrawLength))
  (bind _returnvalue (Class|KismetSystemLibrary|GetTimerElapsedTimeHandle _drawlength))
  (bind _returnvalue_2 (Math|Float|MapRangeClamped _returnvalue 0.0 1.5 1.0 0.2))
  (|CallParentFunction DeltaSeconds)
  (if (and (Variables|Default|GetDrawingString) (Utilities|Time|IsTimerActivebyHandle _drawlength))
    (bind _output_get (Variables|Default|SetDrawPower (Math|Float|MapRangeClamped _returnvalue 0.0 1.5 0.0 1.0)))
    (Class|SOLWeaponsInterface|DrawStrength(Message) (Components|SkeletalMesh|GetAnimInstance (Variables|Default|GetWeapon%20SKM)) _output_get)
    (Variables|Default|SetStandard%20Accuracy (* (Variables|Default|GetRoot%20Accuracy) _returnvalue_2))
    (Variables|Default|SetADS%20Accuracy (* (Variables|Default|GetRoot%20ADS%20Accuracy) _returnvalue_2))))

(event EventPlayerAttemptingWeaponTrigger
  (params (Input%20Status%20From%20Controller :type Boolean))
  (|CallParentFunction Input%20Status%20From%20Controller))

(fn ConstructionScript
  (|CallParentFunction))

(fn AddNiagraVFXtoWeaponMesh
  (params (WeaponMesh :type Skeletal%20Mesh%20Component%20Object%20Reference))
  ;[0.15 0.15 0.15 0.5] Add Muzzle Flash
  (for _array_element (Transformation|GetAllSocketNames (Variables|Default|GetWeapon%20SKM))
    (if (Utilities|String|Contains (Utilities|String|ToString(Name) _array_element) "Muzzle")
      (bind _returnvalue (AddComponent|AddNiagaraComponent false (Math|Transform|MakeTransform "0, 0, 0" "0, 0, 0" (Math|Conversions|ToVector(Float) 0.0035))))
      (Class|NiagaraComponent|SetAsset _returnvalue "/Game/VFX/MuzzleFlashes/Muzzle_Flash.Muzzle_Flash" true)
      (Transformation|AttachComponentToComponent _returnvalue (Variables|Default|GetWeapon%20SKM) _array_element "SnapToTarget" "SnapToTarget" "KeepRelative" true)
      (Utilities|Array|Add (Variables|Default|GetMuzzleFlashArray) _returnvalue)))
  ;[0.15 0.15 0.15 0.5] Add Lasers
  (for _array_element_2 (Transformation|GetAllSocketNames (Variables|Default|GetWeapon%20SKM))
    (if (Utilities|String|Contains (Utilities|String|ToString(Name) _array_element_2) "Laser")
      (bind _returnvalue_2 (AddComponent|AddNiagaraComponent false))
      (Transformation|AttachComponentToComponent _returnvalue_2 (Variables|Default|GetWeapon%20SKM) _array_element_2 "SnapToTarget" "SnapToTarget" "KeepRelative" true)
      (Transformation|AttachComponentToComponent (Variables|Default|GetSpotLight) (Variables|Default|GetWeapon%20SKM) _array_element_2 "SnapToTarget" "SnapToTarget" "KeepRelative" true)
      (Transformation|AttachComponentToComponent (Variables|Default|GetDecal) (Variables|Default|GetWeapon%20SKM) _array_element_2 "SnapToTarget" "SnapToTarget" "KeepRelative" true))))

(fn InitialiseAnimation
  (|CallParentFunction))

(fn SpawnEntityProjectile
  (params (Mesh%20Reference%20To%20Spawn%20From :type Scene%20Component%20Object%20Reference) (SocketMethodTemp :type Name :default "None"))
  (for _index (range 1 12)
    (|CallParentFunction Mesh%20Reference%20To%20Spawn%20From SocketMethodTemp))
  (Camera|PlayWorldCameraShake "/Game/VFX/Camera_Shakes/Shotgun.Shotgun_C" "0, 0, 0" 1e+04 5e+04)
  (Audio|PlaySound2D "/Game/Actors_And_Blueprints/PLAYER/Equipment_Modules/Weapons/HeavyCannon/AC_SFX.AC_SFX" (Math|Random|RandomFloatinRange 0.9 1.1) (Math|Random|RandomFloatinRange 1.9 2.1) 0.0 0 0))

(fn SpawnFLECSProjectile
  (params (Mesh%20Reference%20To%20Spawn%20From :type Scene%20Component%20Object%20Reference) (SocketMethodTemp :type Name :default "None"))
  (bind _returnvalue (Game|GetPlayerController 0))
  (bind _returnvalue_2 (Viewport|GetViewportSize))
  (bind _weapon_skm (Variables|Default|GetWeapon%20SKM))
  (bind _crosshair (Variables|Default|GetCrosshair))
  (bind _returnvalue_3 (Transformation|GetSocketTransform _weapon_skm "None" "RTS_World"))
  (bind _returnvalue_4 (/ _returnvalue_2 "(X=2.000000,Y=2.000000)"))
  (bind _centrecrosshair (Variables|/Game/Actors_And_Blueprints/PLAYER/UI/DynamicCrosshair.DynamicCrosshair_C|GetCentreCrosshair _crosshair))
  (bind _rendertransform (Variables|/Script/UMG.Widget|GetRenderTransform _centrecrosshair))
  (bind _returnvalue_5 (+ (.translation _rendertransform) _returnvalue_4))
  (bind (_worldposition _worlddirection) (Class|GameplayStatics|DeprojectScreentoWorld _returnvalue _returnvalue_5))
  (Camera|PlayWorldCameraShake "/Game/VFX/Camera_Shakes/GrenadeLauncher.GrenadeLauncher_C" "0, 0, 0" 1e+04 5e+04)
  (Audio|PlaySound2D "/Game/Actors_And_Blueprints/PLAYER/Equipment_Modules/Weapons/HeavyCannon/AC_SFX.AC_SFX" (Math|Random|RandomFloatinRange 0.9 1.1) (Math|Random|RandomFloatinRange 1.9 2.1) 0.0 0 0)
  (bind (_outhit _returnvalue_6) (Collision|LineTraceByChannel _worldposition (+ _worldposition (* _worlddirection 1e+04)) "TraceTypeQuery1" false (Utilities|Array|MakeArray (Game|Player|GetPlayerPawn 0)) "None"))
  (Game|SpawnActorfromClass "/Game/Actors_And_Blueprints/PLAYER/Equipment_Modules/Weapons/Projectiles/Bullets/Bolt.Bolt_C" (Math|Transform|MakeTransform (+ (.location _returnvalue_3) (* (Math|Vector|GetForwardVector (Math|Rotator|FindLookatRotation (.location _returnvalue_3) (Math|Vector|SelectVector (.Location (Collision|BreakHitResult _outhit)) (.TraceEnd (Collision|BreakHitResult _outhit)) _returnvalue_6))) 1e+01)) (Math|Rotator|FindLookatRotation (.location _returnvalue_3) (Math|Vector|SelectVector (.Location (Collision|BreakHitResult _outhit)) (.TraceEnd (Collision|BreakHitResult _outhit)) _returnvalue_6)) "1.000000,1.000000,1.000000") "Undefined" "MultiplyWithRoot" 0 (Variables|Default|GetDrawPower) 5.0 0 "Enemy" 4e+01 "Player" 0))