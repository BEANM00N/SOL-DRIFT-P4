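; BP_Dam_Door is an interactable blast door that opens only when the player's inventory holds a Dam_Key.
; A successful interaction runs once, turning the indicator planes and light amber, playing a slow opening montage with camera shake, disabling the cube's collision and showing a message widget.
; A montage notify switches the indicators to green, stops the shake source and fires another shake.
; Without the key, the HUD's interaction widget signals failure.
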(event Collision|EventActorBeginOverlap
  (params (OtherActor :type Actor%20Object%20Reference))
  (|CallParentFunction OtherActor) ; This node is disabled and will not be called.\nDrag off pins to build functionality.
)

(event EventTick
  (params (DeltaSeconds :type Float%20%28single-precision%29))
  (|CallParentFunction DeltaSeconds) ; This node is disabled and will not be called.\nDrag off pins to build functionality.
)

(event EventObjectInteractedwith
  (params (Interaction%20State :type Boolean) (Intigator :type Pawn%20Object%20Reference))
  (if Interaction%20State
    (for _array_element (Variables|/Game/BP_DATA/SOL_Inst_Core.SOL_Inst_Core_C|GetPlayer_Inventory (.AsSOL%20Inst%20Core (Utilities|Casting|CastToSOL_Inst_Core (Game|GetGameInstance))))
      (if (== (Utilities|GetClass _array_element) "/Game/Actors_And_Blueprints/Interactables/ITEMS/PARTS/Dam_Key.Dam_Key_C")
        (Variables|Default|SetKeyFound true)
        (Utilities|DoOnce false
          (:Completed
            (Rendering|Material|SetMaterial (Variables|Default|GetPlane2) 0 "/Game/Actors_And_Blueprints/PLAYER/Equipment_Modules/Weapons/Projectiles/Assets/Materials/MI_Projectile_Yellow.MI_Projectile_Yellow")
            (Rendering|Components|Light|SetLightColor (Variables|Default|GetPointLight) "(R=1.000000,G=0.456411,B=0.000000,A=1.000000)" true)
            (Animation|Montage|PlayMontage (Variables|Default|GetBlastDoors) "/Game/Worlds_And_Levels/Assets/Door/ChamberDoor_Open_Montage.ChamberDoor_Open_Montage" 0.1 0.0 "None" false
              (:then
                (Camera|PlayWorldCameraShake "/Game/VFX/Camera_Shakes/Legacy_Shaker_Light.Legacy_Shaker_Light_C" (Transformation|GetActorLocation) 3e+03 3e+03 0.2)
                (CameraShake|Start (Variables|Default|GetCameraShakeSource))
                (Collision|SetCollisionEnabled (Variables|Default|GetCube) "NoCollision")
                (bind _returnvalue (UserInterface|CreateWidget "/Game/UI/UI_Message.UI_Message_C"))
                (UserInterface|Viewport|AddtoViewport _returnvalue 0))
              (:OnNotifyBegin
                (Rendering|Material|SetMaterial (Variables|Default|GetPlane2) 0 "/Game/Actors_And_Blueprints/AI/Enemies/Enemies/Materials/GREEN_Flash.GREEN_Flash")
                (Rendering|Components|Light|SetLightColor (Variables|Default|GetPointLight) "(R=0.481380,G=1.000000,B=0.000000,A=1.000000)" true)
                (CameraShake|StopAllCameraShakes (Variables|Default|GetCameraShakeSource) false)
                (Camera|PlayWorldCameraShake "/Game/VFX/Camera_Shakes/Legacy_Shaker_Light.Legacy_Shaker_Light_C" (Transformation|GetActorLocation) 3e+03 3e+03 0.2)))))))
    (if (not (Variables|Default|GetKeyFound))
      (Default|InteractionFailed (Variables|/Game/BP_DATA/SOL_HUD_Core.SOL_HUD_Core_C|GetInteraction%20Widget (.AsSOL%20HUD%20Core (Utilities|Casting|CastToSOL_HUD_Core (HUD|GetHUD (Game|GetPlayerController 0)))))))))

(fn ConstructionScript
  (|CallParentFunction))