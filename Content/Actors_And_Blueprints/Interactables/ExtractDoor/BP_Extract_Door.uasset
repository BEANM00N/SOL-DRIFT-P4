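; Interactable extraction door that lets the player end the current game and return to the spawn room level.
; Interacting turns its indicators yellow and enables two initially disabled trigger boxes.
; One box reports extraction attempts to the game mode and binds its extracted event to the blast door opening montage, whose notify turns indicators green.
; The other flags the game as concluded on the game instance and opens the spawn room.
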(event OnComponentBeginOverlap(Box)
  (params (OverlappedComponent :type Primitive%20Component%20Object%20Reference) (OtherActor :type Actor%20Object%20Reference) (OtherComp :type Primitive%20Component%20Object%20Reference) (OtherBodyIndex :type Integer) (bFromSweep :type Boolean) (SweepResult :type Hit%20Result%20Structure%20%28by%20ref%29))
  (if (== OtherActor (Game|Player|GetPlayerPawn 0))
    (bind _assol_inst_core (Utilities|Casting|CastToSOL_Inst_Core (Game|GetGameInstance)))
    (Variables|/Game/BP_DATA/SOL_Inst_Core.SOL_Inst_Core_C|SetGame%20Was%20Concluded _assol_inst_core true)
    (Game|OpenLevel(byObjectReference) "/Game/Worlds_And_Levels/Home/SpawnRoom.SpawnRoom")))

(event OnComponentBeginOverlap(Box1)
  (params (OverlappedComponent :type Primitive%20Component%20Object%20Reference) (OtherActor :type Actor%20Object%20Reference) (OtherComp :type Primitive%20Component%20Object%20Reference) (OtherBodyIndex :type Integer) (bFromSweep :type Boolean) (SweepResult :type Hit%20Result%20Structure%20%28by%20ref%29))
  (if (== OtherActor (Game|Player|GetPlayerPawn 0))
    (bind _assol_game_mode_core (Utilities|Casting|CastToSOL_GameMode_CORE (Game|GetGameMode)))
    (Default|PlayerAttemptingtoExtract _assol_game_mode_core true)
    (EventDispatchers|BindEventtoPlayerExtracted _assol_game_mode_core (delegate Custom|OpenDoor))))

(event OnComponentEndOverlap(Box1)
  (params (OverlappedComponent :type Primitive%20Component%20Object%20Reference) (OtherActor :type Actor%20Object%20Reference) (OtherComp :type Primitive%20Component%20Object%20Reference) (OtherBodyIndex :type Integer))
  (if (== OtherActor (Game|Player|GetPlayerPawn 0))
    (Default|PlayerAttemptingtoExtract (stale OnComponentBeginOverlap(Box1) _assol_game_mode_core) false)))

(event Custom|OpenDoor
  (Animation|Montage|PlayMontage (Variables|Default|GetBlastDoors) "/Game/Worlds_And_Levels/Assets/Door/ChamberDoor_Open_Montage.ChamberDoor_Open_Montage" 1.0 0.0 "None" false
    (:OnNotifyBegin
      (Rendering|Material|SetMaterial (Variables|Default|GetPlane2) 0 "/Game/Actors_And_Blueprints/AI/Enemies/Enemies/Materials/GREEN_Flash.GREEN_Flash")
      (Rendering|Components|Light|SetLightColor (Variables|Default|GetPointLight) "(R=0.481380,G=1.000000,B=0.000000,A=1.000000)" true))))

(event EventBeginPlay
  (|CallParentFunction)
  (Collision|SetCollisionEnabled (Variables|Default|GetBox) "NoCollision"))

(event Collision|EventActorBeginOverlap
  (params (OtherActor :type Actor%20Object%20Reference))
  (|CallParentFunction OtherActor) ; This node is disabled and will not be called.\nDrag off pins to build functionality.
)

(event EventTick
  (params (DeltaSeconds :type Float%20%28single-precision%29))
  (|CallParentFunction DeltaSeconds) ; This node is disabled and will not be called.\nDrag off pins to build functionality.
)

(event EventObjectInteractedwith
  (params (Interaction%20State :type Boolean) (Intigator :type Pawn%20Object%20Reference))
  (Rendering|Material|SetMaterial (Variables|Default|GetPlane2) 0 "/Game/Actors_And_Blueprints/PLAYER/Equipment_Modules/Weapons/Projectiles/Assets/Materials/MI_Projectile_Yellow.MI_Projectile_Yellow")
  (Rendering|Components|Light|SetLightColor (Variables|Default|GetPointLight) "(R=1.000000,G=0.456411,B=0.000000,A=1.000000)" true)
  (Collision|SetCollisionEnabled (Variables|Default|GetBox) "QueryOnly"))

(fn ConstructionScript
  (|CallParentFunction))