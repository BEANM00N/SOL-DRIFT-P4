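; BP_Chest is an interactable chest that is replaced by a ChainRaptorInteractableBase pickup when used.
; From BeginPlay, the Flash timeline restarts itself endlessly, driving the particle system's scale from zero to a very large size as a pulsing effect.
; ObjectInteractedwith spawns the pickup at the chest's location, calls CallInteractedWith and destroys the chest.
; Disconnected leftover nodes for a controls-guide widget and a DMR spawn never run.
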(event Custom|Flash%20Event
  (bind _alpha (Timeline|Flash PlayFromStart)
    (:Update
      (Transformation|SetRelativeScale3D (Variables|Default|GetParticleSystem) (Math|Conversions|ToVector(Float) (Math|Float|Lerp 0.0 1e+04 _alpha))))
    (:Finished
      (CallFunction|FlashEvent))))

(event EventBeginPlay
  (CallFunction|FlashEvent))

(event Collision|EventActorBeginOverlap
  (params (OtherActor :type Actor%20Object%20Reference)))

(event EventTick
  (params (DeltaSeconds :type Float%20%28single-precision%29)))

(event EventObjectInteractedwith
  (params (Interaction%20State :type Boolean))
  (Game|SpawnActorfromClass "/Game/Actors_And_Blueprints/Pickups/Weapon/ChainRaptorInteractableBase.ChainRaptorInteractableBase_C" (Math|Transform|MakeTransform (+ (Transformation|GetActorLocation) "") "0, 0, 0" "1.000000,1.000000,1.000000") "Undefined" "MultiplyWithRoot" 0 0)
  (Default|CallInteractedwith)
  (Actor|DestroyActor))

(fn ConstructionScript)