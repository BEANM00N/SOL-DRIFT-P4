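; Interactable extraction terminal that calls in an extraction pod, presented to players as a "Diving Cage".
; The first positive interaction spawns BP_ExtractionPod far below the world origin with a random yaw, guarded by a DoOnce.
; It passes the parent actor's location as the pod's zone location, so the terminal relies on having a parent actor, along with the pod's name and interaction prompt.
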(event EventBeginPlay
  (|CallParentFunction))

(event Collision|EventActorBeginOverlap
  (params (OtherActor :type Actor%20Object%20Reference))
  (|CallParentFunction OtherActor) ; This node is disabled and will not be called.\nDrag off pins to build functionality.
)

(event EventTick
  (params (DeltaSeconds :type Float%20%28single-precision%29))
  (|CallParentFunction DeltaSeconds) ; This node is disabled and will not be called.\nDrag off pins to build functionality.
)

(event EventObjectInteractedwith
  (params (Interaction%20State :type Boolean) (Intigator :type Object%20Object%20Reference))
  (if Interaction%20State
    (Utilities|DoOnce false
      (:Completed
        (Game|SpawnActorfromClass "/Game/Worlds_And_Levels/Assets/Extraction/BP_ExtractionPod.BP_ExtractionPod_C" (Math|Transform|MakeTransform "0.000000,0.000000,-10000.000000" (Math|Rotator|MakeRotator 0.0 0.0 (Math|Random|RandomFloatinRange 0.0 3.6e+02)) "1.000000,1.000000,1.000000") "Undefined" "MultiplyWithRoot" 0 (Transformation|GetActorLocation (Actor|GetParentActor self)) "Begin Extraction" "Diving Cage" 0)))))

(fn ConstructionScript
  (|CallParentFunction))