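; BP_ExtractionPod is an extraction pod that drops from high above a zone location, then loads the spawn room level when interacted with.
; A Drop timeline lerps it down while Tick flickers the lens flare and moves a marker on a distance widget.
; On landing it triggers crash effects, rubble, spotlights and a camera shake, then stops ticking.
; The construction script stacks alternately rotated chain link instances to a set length.
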(event EventBeginPlay
  (bind _returnvalue (UserInterface|CreateWidget "/Game/Worlds_And_Levels/Assets/Extraction/UI_ExtractionDistance.UI_ExtractionDistance_C"))
  (UserInterface|Viewport|AddtoViewport _returnvalue 0)
  (Variables|Default|SetAs%20UI%20Extraction%20Distance _returnvalue)
  (Variables|Default|SetSpawnLocation (+ (Variables|Default|GetZoneLocation) "0.000000,0.000000,1000000.000000"))
  (Variables|Default|SetZoneLocation (+ (Variables|Default|GetZoneLocation) "0.000000,0.000000,200.000000"))
  (bind _alpha (Timeline|Drop PlayFromStart)
    (:Update
      (Transformation|SetActorLocation (Math|Vector|Lerp(Vector) (Variables|Default|GetSpawnLocation) (Variables|Default|GetZoneLocation) _alpha) false false))
    (:Finished
      (Components|Activation|Activate (Variables|Default|GetNS_ExtractionCrash) false)
      (Rendering|SetVisibility (Variables|Default|GetPodRubble1) true false)
      (Rendering|SetVisibility (Variables|Default|GetLensFlare) false false)
      (Camera|PlayWorldCameraShake "/Game/VFX/Camera_Shakes/Legacy_Shaker_baker.Legacy_Shaker_baker_C" (Transformation|GetActorLocation) 3e+04 3e+04 0.2)
      (Actor|Tick|SetActorTickEnabled false))))

(event Collision|EventActorBeginOverlap
  (params (OtherActor :type Actor%20Object%20Reference)))

(event EventTick
  (params (DeltaSeconds :type Float%20%28single-precision%29))
  (Transformation|SetRelativeScale3D (Variables|Default|GetLensFlare) (Math|Conversions|ToVector(Float) (Math|Random|RandomFloatinRange 1e+01 3e+01)))
  (Class|Widget|SetRenderTranslation (Variables|/Game/Worlds_And_Levels/Assets/Extraction/UI_ExtractionDistance.UI_ExtractionDistance_C|GetPositionBox (Variables|Default|GetAs%20UI%20Extraction%20Distance)) (Math|Vector2D|MakeVector2D (Math|Float|MapRangeClamped (Math|Vector|Distance(Vector) (Transformation|GetActorLocation) (Variables|Default|GetZoneLocation)) (.z (Variables|Default|GetSpawnLocation)) (.z (Variables|Default|GetZoneLocation)) -1e+01 3.9e+02) 0.0)))

(event EventObjectInteractedwith
  (params (Interaction%20State :type Boolean) (Intigator :type Object%20Object%20Reference))
  (Game|OpenLevel(byObjectReference) "/Game/Worlds_And_Levels/Home/SpawnRoom.SpawnRoom"))

(fn ConstructionScript
  (for _index (range 0 (Math|Float|Truncate (/ (Variables|Default|GetChainLength) 85.0)))
    (Components|InstancedStaticMesh|AddInstance (Variables|Default|GetChainLink) (Math|Transform|MakeTransform (Variables|Default|GetInstance%20Transform%20Location) (Variables|Default|GetInstance%20Transform%20Rotation) "1.000000,1.000000,1.000000") false)
    (Variables|Default|SetInstance%20Transform%20Location (Math|Vector|MakeVector 0.0 0.0 (+ (.z (Variables|Default|GetInstance%20Transform%20Location)) 85.0)))
    (Variables|Default|SetInstance%20Transform%20Rotation (Math|Rotator|MakeRotator 0.0 0.0 (+ (.yaw (Variables|Default|GetInstance%20Transform%20Rotation)) 9e+01)))))