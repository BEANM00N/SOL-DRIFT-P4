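; Orbit camera pawn that takes over player control, with mouse-driven rotation and zoom around a spring arm.
; BeginPlay unpossesses and calls destroy on the player controller, aims the arm toward the player pawn's location, then possesses itself.
; Possession blends the view and adds the IMC_Whale input mapping.
; Tick interpolates arm length from scroll input and pitch/yaw from mouse delta while right-click is held (stored as LeftClickHeld).
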(event Input|EnhancedActionEvents|EnhancedInputActionMouse_Click-Right
  (params (ActionValue :type Boolean) (ElapsedSeconds :type Float%20%28double-precision%29) (TriggeredSeconds :type Float%20%28double-precision%29) (InputAction :type Input%20Action%20Object%20Reference :default "/Game/Actors_And_Blueprints/PLAYER/Input/Actions/Weapons/Mouse_Click-Right.Mouse_Click-Right"))
  (:Started
    (Variables|Default|SetLeftClickHeld ActionValue :!label _label))
  (:Canceled
    (goto _label))
  (:Completed
    (goto _label)))

(event Input|EnhancedActionEvents|EnhancedInputActionMouse_Scroll
  (params (ActionValue :type Float%20%28double-precision%29) (ElapsedSeconds :type Float%20%28double-precision%29) (TriggeredSeconds :type Float%20%28double-precision%29) (InputAction :type Input%20Action%20Object%20Reference :default "/Game/Actors_And_Blueprints/PLAYER/Input/Actions/Mouse_Scroll.Mouse_Scroll"))
  (:Triggered
    (Variables|Default|SetMouseScroll ActionValue))
  (:Completed
    (Variables|Default|SetMouseScroll 0.0)))

(event EventBeginPlay
  (bind _returnvalue (Game|GetPlayerController 0))
  (Pawn|UnPossess _returnvalue)
  (Actor|DestroyActor _returnvalue)
  (Transformation|SetRelativeRotation (Variables|Default|GetSpringArm) (Math|Rotator|FindLookatRotation (Transformation|GetActorLocation) (Transformation|GetActorLocation (Game|Player|GetPlayerPawn 0))) false false)
  (Pawn|Possess (Game|GetPlayerController 0) self))

(event Collision|EventActorBeginOverlap
  (params (OtherActor :type Actor%20Object%20Reference)))

(event EventPossessed
  (params (NewController :type Controller%20Object%20Reference))
  (Game|Player|SetViewTargetwithBlend (Game|GetPlayerController 0) self 0.5 "VTBlend_EaseInOut" 0.0 false)
  (Input|AddMappingContext (PlayerController|LocalPlayerSubsystems|GetEnhancedInputLocalPlayerSubsystem (Game|GetPlayerController 0)) "/Game/Actors_And_Blueprints/PLAYER/Input/Actions/Whale/IMC_Whale.IMC_Whale" 0 "(bIgnoreAllPressedKeysUntilRelease=True,bForceImmediately=False,bNotifyUserSettings=False)")
  (Input|EnableInput (Game|GetPlayerController 0)))

(event EventTick
  (params (DeltaSeconds :type Float%20%28single-precision%29))
  (bind _returnvalue (Game|GetPlayerController 0))
  (bind _springarm (Variables|Default|GetSpringArm))
  (bind _springarm_2 (Variables|Default|GetSpringArm))
  (bind (_deltax _deltay) (Class|PlayerController|GetInputMouseDelta _returnvalue))
  (bind _relativerotation (Variables|/Script/Engine.SceneComponent|GetRelativeRotation _springarm))
  (bind _returnvalue_2 (Math|Vector2D|MakeVector2D _deltax _deltay))
  (bind _returnvalue_3 (Math|Vector2D|MakeVector2D (.yaw _relativerotation) (.pitch _relativerotation)))
  (bind _returnvalue_4 (* _returnvalue_2 5e+01))
  (bind _returnvalue_5 (+ _returnvalue_3 _returnvalue_4))
  (bind _returnvalue_6 (Class|KismetMathLibrary|Vector2DInterpto _returnvalue_3 _returnvalue_5 DeltaSeconds 1.0))
  (bind (_x _y) (Math|Vector2D|BreakVector2D _returnvalue_6))
  (Variables|/Script/Engine.SpringArmComponent|SetTargetArmLength _springarm_2 (Math|Interpolation|FInterpTo (Variables|/Script/Engine.SpringArmComponent|GetTargetArmLength _springarm_2) (+ (Variables|/Script/Engine.SpringArmComponent|GetTargetArmLength _springarm_2) (* (Variables|Default|GetMouseScroll) -5e+03)) DeltaSeconds 1.0))
  (if (Variables|Default|GetLeftClickHeld)
    (Transformation|SetRelativeRotation (Variables|Default|GetSpringArm) (Math|Rotator|MakeRotator 0.0 _y _x) false false)))

(fn ConstructionScript)