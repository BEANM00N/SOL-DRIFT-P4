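; BP_Chain is a chain prop that builds instanced links along a spline in its construction script.
; Link count follows spline length, with roll stepped 90 degrees per link to alternate orientation.
; Each position divides spline length by the index, so spacing is uneven, and world-space locations feed AddInstance.
; A disconnected loop would scroll links along the spline by a distance offset, but nothing runs at play time.
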(event EventBeginPlay)

(event Collision|EventActorBeginOverlap
  (params (OtherActor :type Actor%20Object%20Reference)))

(event EventTick
  (params (DeltaSeconds :type Float%20%28single-precision%29)))

(fn ConstructionScript
  (bind _spline (Variables|Default|GetSpline))
  (bind _returnvalue (Spline|GetSplineLength _spline))
  (for _index (range 0 (Math|Float|Floor (/ _returnvalue 7e+01)))
    (Components|InstancedStaticMesh|AddInstance (Variables|Default|GetChainLink) (Math|Transform|MakeTransform (.location (Spline|GetTransformatDistanceAlongSpline (Variables|Default|GetSpline) (/ _returnvalue _index) "World" false)) (Variables|Default|GetChain%20Rotation) "1.000000,1.000000,1.000000") false)
    (Variables|Default|SetChain%20Rotation (Math|Rotator|MakeRotator (+ (.roll (Variables|Default|GetChain%20Rotation)) 9e+01) (.pitch (Variables|Default|GetChain%20Rotation)) (.yaw (Variables|Default|GetChain%20Rotation))))))